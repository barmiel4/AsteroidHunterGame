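; BP_UltraBolt is a player gun projectile that hits asteroids and scatters mines.
; When its Sphere overlaps a BP_Asteroid, it calls that asteroid's OnCollision, then runs SpawnMines.
; SpawnMines loops over adjacent yaw sectors, spawning one BP_Mine in each at the bolt's location and scale with a random yaw, forming a jittered fan that leaves a gap short of a full circle.
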(event `self.ReceiveBeginPlay`
  (`parent.ReceiveBeginPlay`))

(event `self.Sphere.OnComponentBeginOverlap`
  (params (OverlappedComponent :type "PrimitiveComponent Object Reference") (OtherActor :type "Actor Object Reference") (OtherComp :type "PrimitiveComponent Object Reference") (OtherBodyIndex :type Integer) (bFromSweep :type Boolean) (SweepResult :type "HitResult Structure (by ref)"))
  (bind _asbp_asteroid (cast `/Game/Blueprints/Obstacles/BP_Asteroid` OtherActor))
  (`/Game/Blueprints/Obstacles/BP_Asteroid.OnCollision` _asbp_asteroid 0)
  (`self.SpawnMines`))

(fn `SpawnMines`
  (for _index (range -4 4)
    (bind _returnvalue (`KismetMathLibrary.Conv_IntToDouble` _index))
    (`|SpawnActorFromClass` "/Game/Blueprints/Player/GUNS/BP_Mine.BP_Mine_C" (`KismetMathLibrary.MakeTransform` (`self.K2_GetActorLocation`) (`KismetMathLibrary.MakeRotator` 0.0 0.0 (* (`KismetMathLibrary.RandomFloatInRange` _returnvalue (+ _returnvalue 1.0)) 36.0)) (`self.GetActorScale3D`)) "Undefined" "OverrideRootScale" null null)))

(fn `UserConstructionScript`
  (`parent.UserConstructionScript`))