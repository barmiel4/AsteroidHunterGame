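; BP_Mine is a mine that launches itself a random distance forward when spawned and disappears when its mesh is overlapped.
; A BeginPlay timeline eases its location from just above the spawn point, with a second track scaling a Bump offset along the way.
; Tick pulses a dynamic material's color between yellow and red.
; Overlap only destroys the actor and prints a note that the intended points are not awarded.
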(event `self.ReceiveBeginPlay`
  (bind _start (`self.Start`))
  (bind _returnvalue (`PrimitiveComponent.CreateDynamicMaterialInstance` (`self.Mine Mesh`) 0 "/Game/Materials/M_Mine.M_Mine" "None"))
  (set `self.Material` _returnvalue)
  (set `self.Start` (+ (`self.K2_GetActorLocation`) (0.0 0.0 10.0)))
  (set `self.RandomDistance` (`KismetMathLibrary.RandomFloatInRange` 170.0 300.0))
  (bind (_direction _alpha _alphaz) (`Timeline|Spawn Position Fade` :!via `PlayFromStart`)
    (:`Update`
      (`self.K2_SetActorLocation` (`|EaseFunction` "EaseInOut" _alpha _start (+ _start (* (`self.GetActorForwardVector`) (`self.RandomDistance`)) (* (`self.Bump`) _alphaz)))))))

(event `self.ReceiveTick`
  (params (DeltaSeconds :type "Float (single-precision)"))
  (`MaterialInstanceDynamic.SetVectorParameterValue` (`self.Material`) "Color" (`KismetMathLibrary.LinearColorLerp` (struct :`R` 10.0 :`G` 9.456426 :`A` 1.0) (struct :`R` 1.0 :`B` 0.07036 :`A` 1.0) (`KismetMathLibrary.MakePulsatingValue` (`KismetSystemLibrary.GetGameTimeInSeconds`) 2.0))))

(event `self.Mine Mesh.OnComponentBeginOverlap`
  (params (OverlappedComponent :type "PrimitiveComponent Object Reference") (OtherActor :type "Actor Object Reference") (OtherComp :type "PrimitiveComponent Object Reference") (OtherBodyIndex :type Integer) (bFromSweep :type Boolean) (SweepResult :type "HitResult Structure (by ref)"))
  (`self.K2_DestroyActor`)
  (`KismetSystemLibrary.PrintString` "mines should give 2 points, they dont" true true (struct :`R` 1.0 :`B` 0.050978 :`A` 1.0)))

(fn `UserConstructionScript`)