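; BP_DefaultBolt is a gun projectile that awards the player's P_HeroSpaceship points when it hits a target.
; Mesh overlaps with GameTraceChannel1 objects add score and optionally destroy the bolt.
; SetUpProjectile applies a given speed along the actor's forward vector.
; TriggerChaosExplosion, not called within this Blueprint, spawns a temporary FS_MasterField at the bolt, fires a strain-only Chaos pulse, then destroys the field.
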(event `self.ReceiveBeginPlay`
  (bind _asp_hero_spaceship (cast `/Game/Blueprints/Player/P_HeroSpaceship` (`GameplayStatics.GetPlayerPawn` 0)))
  (set `self.Player Reference` _asp_hero_spaceship))

(event `self.BoltMesh.OnComponentBeginOverlap`
  (params (OverlappedComponent :type "PrimitiveComponent Object Reference") (OtherActor :type "Actor Object Reference") (OtherComp :type "PrimitiveComponent Object Reference") (OtherBodyIndex :type Integer) (bFromSweep :type Boolean) (SweepResult :type "HitResult Structure (by ref)"))
  (if (`|EnumEquality` (`PrimitiveComponent.GetCollisionObjectType` OtherComp) "ECC_GameTraceChannel1")
    (`/Game/Blueprints/Player/P_HeroSpaceship.IncreaseScore` (`self.Player Reference`) (`self.PointsOnImpact`))
    (if (`self.DestoyOnImpact`)
      (`self.K2_DestroyActor`))))

(fn `SetUpProjectile`
  (params (`Bolt Speed` :type "Float (single-precision)"))
  (bind _projectilemovement (`self.ProjectileMovement`))
  (bind _projectilemovement_2 (`self.ProjectileMovement`))
  (bind _output_get (set `ProjectileMovementComponent.MaxSpeed` `Bolt Speed` _projectilemovement))
  (set `ProjectileMovementComponent.InitialSpeed` _output_get _projectilemovement)
  (set `MovementComponent.Velocity` (* (`ProjectileMovementComponent.InitialSpeed` _projectilemovement_2) (`self.GetActorForwardVector`)) _projectilemovement_2))

(fn `Trigger Chaos Explosion`
  (bind _returnvalue (`|SpawnActorFromClass` "/Engine/EditorResources/FieldNodes/FS_MasterField.FS_MasterField_C" (`KismetMathLibrary.Conv_VectorToTransform` (`self.K2_GetActorLocation`)) "Undefined" "MultiplyWithRoot" null null))
  (set `/Engine/EditorResources/FieldNodes/FS_MasterField.Radial Magnitude` 0.0 _returnvalue)
  (set `/Engine/EditorResources/FieldNodes/FS_MasterField.Strain Magnitude` 500000.0 _returnvalue)
  (`/Engine/EditorResources/FieldNodes/FS_MasterField.CE_Trigger` _returnvalue)
  (`self.K2_DestroyActor` _returnvalue))

(fn `UserConstructionScript`)