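; BP_Rifle is a rifle projectile that hits asteroids, moved by a ProjectileMovement component.
; When its Sphere overlaps a BP_Asteroid, it calls that asteroid's OnCollision and destroys itself, ignoring other actors.
; BeginPlay runs the parent logic, then prints the projectile's speed for debugging.
; A leftover randomized-speed setup is disconnected and never runs.
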(event `self.ReceiveBeginPlay`
  (`parent.ReceiveBeginPlay`)
  (`KismetSystemLibrary.PrintString` (`KismetStringLibrary.Concat_StrStr` "rifle speed" (`KismetStringLibrary.Conv_DoubleToString` (`KismetMathLibrary.VSize` (`MovementComponent.Velocity` (`self.ProjectileMovement`)))))))

(event `self.Sphere.OnComponentBeginOverlap`
  (params (OverlappedComponent :type "PrimitiveComponent Object Reference") (OtherActor :type "Actor Object Reference") (OtherComp :type "PrimitiveComponent Object Reference") (OtherBodyIndex :type Integer) (bFromSweep :type Boolean) (SweepResult :type "HitResult Structure (by ref)"))
  (bind _asbp_asteroid (cast `/Game/Blueprints/Obstacles/BP_Asteroid` OtherActor))
  (`/Game/Blueprints/Obstacles/BP_Asteroid.OnCollision` _asbp_asteroid 1)
  (`self.K2_DestroyActor`))

(fn `UserConstructionScript`
  (`parent.UserConstructionScript`))