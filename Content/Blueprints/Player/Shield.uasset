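; Shield component for the player's hero spaceship that tracks shield health and shuts the shield down when depleted.
; Each HandleShield call decrements health or, at zero, disables the mesh's collision and visibility, refills health and sets the player's next score threshold from current score plus shield cost.
; It also lerps the shield material's color from green toward red as health drops.
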(event `self.ReceiveBeginPlay`
  (bind _asp_hero_spaceship (cast `/Game/Blueprints/Player/P_HeroSpaceship` (`self.GetOwner`)))
  (set `self.Player` _asp_hero_spaceship)
  (set `self.Health` (`self.MaxHealth`)))

(fn `HandleShield`
  (bind _player (`self.Player`))
  (bind _player_2 (`self.Player`))
  (`|ExecutionSequence`
    (:`then_0`
      (if (> (`self.Health`) 0.0)
        (`/Engine/EditorBlueprintResources/StandardMacros.DecrementFloat` (`self.Health`))
        (else
          (`PrimitiveComponent.SetCollisionEnabled` (`/Game/Blueprints/Player/P_HeroSpaceship.ShieldMesh` _player_2) "NoCollision")
          (`SceneComponent.SetVisibility` (`/Game/Blueprints/Player/P_HeroSpaceship.ShieldMesh` _player_2) false false)
          (set `self.Health` (`self.MaxHealth`))
          (set `self.Using` false)
          (set `/Game/Blueprints/Player/P_HeroSpaceship.Shield Threshold` (+ (`/Game/Blueprints/Player/P_HeroSpaceship.Shield Cost` _player) (`/Game/Blueprints/Player/P_HeroSpaceship.Score` _player)) (`self.Player`)))))
    (:`then_1`
      (`MaterialInstanceDynamic.SetVectorParameterValue` (`/Game/Blueprints/Player/P_HeroSpaceship.ShieldMaterial` (`self.Player`)) "Color" (`KismetMathLibrary.LinearColorLerp` (struct :`R` 4.0 :`B` 0.037447 :`A` 1.0) (struct :`G` 4.0 :`B` 0.216959 :`A` 1.0) (/ (`self.Health`) (`self.MaxHealth`)))))))