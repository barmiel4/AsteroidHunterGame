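; BP_Shield is a shield actor that follows the player's P_HeroSpaceship by offsetting itself each tick by the ship's velocity, while printing its Health for debugging.
; Asteroids overlapping its sphere spawn a destructible and are destroyed, costing one Health, or destroying the shield if Health is already depleted.
; A dynamic material created in the construction script shifts the shield's color from green toward red as Health drops.
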(event `self.ReceiveBeginPlay`
  (bind _asp_hero_spaceship (cast `/Game/Blueprints/Player/P_HeroSpaceship` (`GameplayStatics.GetPlayerPawn` 0)))
  (set `self.Player` _asp_hero_spaceship))

(event `self.ReceiveTick`
  (params (DeltaSeconds :type "Float (single-precision)"))
  (`KismetSystemLibrary.PrintString` (`KismetStringLibrary.Conv_DoubleToString` (`self.Health`)))
  (`self.K2_AddActorWorldOffset` (* (`self.GetVelocity` (`self.Player`)) DeltaSeconds)))

(event `self.Sphere.OnComponentBeginOverlap`
  (params (OverlappedComponent :type "PrimitiveComponent Object Reference") (OtherActor :type "Actor Object Reference") (OtherComp :type "PrimitiveComponent Object Reference") (OtherBodyIndex :type Integer) (bFromSweep :type Boolean) (SweepResult :type "HitResult Structure (by ref)"))
  (bind _asbp_asteroid (cast `/Game/Blueprints/Obstacles/BP_Asteroid` OtherActor))
  (`/Game/Blueprints/Obstacles/BP_Asteroid.SpawnDestructible` _asbp_asteroid (0.0 0.0 0.0) 80.0 10000.0)
  (`self.K2_DestroyActor` _asbp_asteroid)
  (`|ExecutionSequence`
    (:`then_0`
      (if (> (`self.Health`) 0.0)
        (`/Engine/EditorBlueprintResources/StandardMacros.DecrementFloat` (`self.Health`))
        (else
          (`self.K2_DestroyActor`))))
    (:`then_1`
      (`MaterialInstanceDynamic.SetVectorParameterValue` (`self.DMInstance`) "Color" (`KismetMathLibrary.LinearColorLerp` (struct :`R` 3.0 :`G` 0.007843) (struct :`G` 1.0) (/ (`self.Health`) 10.0))))))

(fn `UserConstructionScript`
  (bind _returnvalue (`PrimitiveComponent.CreateDynamicMaterialInstance` (`self.StaticMesh`) 0 "/Game/Materials/M_Shield.M_Shield" "None"))
  (set `self.DMInstance` _returnvalue))