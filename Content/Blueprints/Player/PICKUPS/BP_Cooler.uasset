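; BP_Cooler is a pickup that cools the player spaceship's gun on overlap, then destroys itself.
; It caches the player's P_HeroSpaceship on BeginPlay and homes in on it every tick, with no range check.
; DetermineLocation uses VInterpTo toward a point offset behind the ship on world X and yaws the pickup to face it.
; The spawn location is stored, but the distance calculation using it is unused.
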(event `self.ReceiveBeginPlay`
  (bind _asp_hero_spaceship (cast `/Game/Blueprints/Player/P_HeroSpaceship` (`GameplayStatics.GetPlayerPawn` 0)))
  (set `self.Player` _asp_hero_spaceship))

(event `self.ReceiveTick`
  (params (DeltaSeconds :type "Float (single-precision)"))
  (set `self.Delta` DeltaSeconds)
  (`self.DetermineLocation`))

(event `self.Collision.OnComponentBeginOverlap`
  (params (OverlappedComponent :type "PrimitiveComponent Object Reference") (OtherActor :type "Actor Object Reference") (OtherComp :type "PrimitiveComponent Object Reference") (OtherBodyIndex :type Integer) (bFromSweep :type Boolean) (SweepResult :type "HitResult Structure (by ref)"))
  (bind _asp_hero_spaceship (cast `/Game/Blueprints/Player/P_HeroSpaceship` OtherActor))
  (`/Game/Blueprints/Player/P_HeroSpaceship.CoolGun` _asp_hero_spaceship)
  (`self.K2_DestroyActor`))

(fn `DetermineLocation`
  (`self.K2_SetActorLocation` (`KismetMathLibrary.VInterpTo` (`self.K2_GetActorLocation`) (`KismetMathLibrary.MakeVector` (- (.x (`self.K2_GetActorLocation` (`self.Player`))) 100.0) (.y (`self.K2_GetActorLocation` (`self.Player`))) (.z (`self.K2_GetActorLocation` (`self.Player`)))) (`self.Delta`) 5.0))
  (`self.K2_SetActorRotation` (`KismetMathLibrary.MakeRotator` (.roll (`self.K2_GetActorRotation`)) (.pitch (`self.K2_GetActorRotation`)) (.yaw (`KismetMathLibrary.FindLookAtRotation` (`self.K2_GetActorLocation`) (`self.K2_GetActorLocation` (`self.Player`)))))))

(fn `UserConstructionScript`
  (set `self.OnSpawnedLocation` (`self.K2_GetActorLocation`)))