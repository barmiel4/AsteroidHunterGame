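; Asteroid obstacle that shatters and destroys itself when the hero spaceship overlaps its sphere.
; The overlap deals damage and triggers the ship's collision reaction unless its shield is in use.
; A separate OnCollision function adds a passed score to the player before destroying the asteroid.
; Both paths fake the breakup by spawning a Destructible at the mesh transform plus a RadialForceActor with path-specific radius and strength.
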(event `self.ReceiveBeginPlay`
  (`parent.ReceiveBeginPlay`)
  (bind _asp_hero_spaceship (cast `/Game/Blueprints/Player/P_HeroSpaceship` (`GameplayStatics.GetPlayerPawn` 0)))
  (set `self.Player` _asp_hero_spaceship))

(event `self.Sphere.OnComponentBeginOverlap`
  (params (OverlappedComponent :type "PrimitiveComponent Object Reference") (OtherActor :type "Actor Object Reference") (OtherComp :type "PrimitiveComponent Object Reference") (OtherBodyIndex :type Integer) (bFromSweep :type Boolean) (SweepResult :type "HitResult Structure (by ref)"))
  (bind _asp_hero_spaceship (cast `/Game/Blueprints/Player/P_HeroSpaceship` OtherActor))
  (`self.SpawnDestructible` (0.0 0.0 0.0) 80.0 10000.0)
  (if (`self.checkShield` _asp_hero_spaceship)
    (`/Game/Blueprints/Player/P_HeroSpaceship.TakeDamage` _asp_hero_spaceship 20.0)
    (`/Game/Blueprints/Player/P_HeroSpaceship.CollisionReaction` _asp_hero_spaceship (`self.K2_GetActorLocation`))
    (`PrimitiveComponent.SetCollisionEnabled` (`self.Sphere`) "NoCollision")
    (`self.K2_DestroyActor`)
    (else
      (`self.K2_DestroyActor`))))

(fn `checkShield`
  (params (Reference :type "/Game/Blueprints/Player/P_HeroSpaceship Object Reference"))
  (returns (ReturnValue :type Boolean))
  (return (not (`/Game/Blueprints/Player/Shield.Using` (`/Game/Blueprints/Player/P_HeroSpaceship.Shield` Reference)))))

(fn `OnCollision`
  (params (score :type Integer))
  (set `/Game/Blueprints/Player/P_HeroSpaceship.Score` (+ (`/Game/Blueprints/Player/P_HeroSpaceship.Score` (`self.player`)) score) (`self.player`))
  (`self.SpawnDestructible` (5.0 0.0 0.0) 85.0 5000.0)
  (`self.K2_DestroyActor`))

(fn `SpawnDestructible`
  (params (Offset :type "Vector Structure") (Radius :type "Float (double-precision)") (Strength :type "Float (double-precision)"))
  (bind _returnvalue (`SceneComponent.K2_GetComponentToWorld` (`self.StaticMesh`)))
  (`|SpawnActorFromClass` "/Game/Blueprints/Obstacles/Destructible.Destructible_C" _returnvalue "AlwaysSpawn" "OverrideRootScale" null null)
  (bind _returnvalue_2 (`|SpawnActorFromClass` "/Script/Engine.RadialForceActor" (`KismetMathLibrary.MakeTransform` (- (.location _returnvalue) Offset)) "AlwaysSpawn" "MultiplyWithRoot" null null))
  (bind _forcecomponent (`RadialForceActor.ForceComponent` _returnvalue_2))
  (set `RadialForceComponent.Radius` Radius _forcecomponent)
  (set `RadialForceComponent.ForceStrength` Strength _forcecomponent))

(fn `UserConstructionScript`
  (`parent.UserConstructionScript`))