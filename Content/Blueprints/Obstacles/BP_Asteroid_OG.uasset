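; Asteroid obstacle that shatters through Chaos destruction when overlapped, damaging and triggering a collision reaction on the hero spaceship.
; Any sphere overlap stops projectile movement, enables Geometry Collection physics, disables sphere collision and schedules destruction after LifeTime.
; The explosion applies external strain and culled radial velocity fields, offset randomly toward the hit actor or cached hit location.
; OnCollision only prints, and older field-actor and debug logic remains disconnected.
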(event `self.ReceiveBeginPlay`
  (`parent.ReceiveBeginPlay`))

(event `self.Sphere.OnComponentBeginOverlap`
  (params (OverlappedComponent :type "PrimitiveComponent Object Reference") (OtherActor :type "Actor Object Reference") (OtherComp :type "PrimitiveComponent Object Reference") (OtherBodyIndex :type Integer) (bFromSweep :type Boolean) (SweepResult :type "HitResult Structure (by ref)"))
  (`self.Handle Collision` OtherActor)
  (bind _asp_hero_spaceship (cast `/Game/Blueprints/Player/P_HeroSpaceship` OtherActor))
  (`/Game/Blueprints/Player/P_HeroSpaceship.TakeDamage` _asp_hero_spaceship 20.0)
  (`/Game/Blueprints/Player/P_HeroSpaceship.Collision Reaction` _asp_hero_spaceship (`self.K2_GetActorLocation`)))

(event `self.Sphere.OnComponentHit`
  (params (HitComponent :type "PrimitiveComponent Object Reference") (OtherActor :type "Actor Object Reference") (OtherComp :type "PrimitiveComponent Object Reference") (NormalImpulse :type "Vector Structure") (Hit :type "HitResult Structure (by ref)")))

(fn `Destroy`
  (`self.K2_DestroyActor`))

(fn `Handle Collision`
  (params (HitActor :type "Actor Object Reference"))
  (locals (`Hit Actor Location` :type "Vector Structure") (NewLocalVar :type "Vector Structure" :default (0.0 0.0 0.0)))
  (`ActorComponent.Deactivate` (`self.ProjectileMovement`))
  (`PrimitiveComponent.SetSimulatePhysics` (`self.GeometryCollection`) true)
  (`PrimitiveComponent.SetCollisionEnabled` (`self.Sphere`) "NoCollision")
  (`KismetSystemLibrary.K2_SetTimer` null "Destroy" (`self.Life Time`))
  (`|ExecutionSequence`
    (:`then_0`
      (bind _hitactor (`local.HitActor`)
        (:`then`
          (set `local.Hit Actor Location` (`self.K2_GetActorLocation` _hitactor)))
        (:`else`
          (set `local.Hit Actor Location` (`self.Hit Location Cache`)))))
    (:`then_1`
      (`self.Trigger Chaos Explosion` (`KismetMathLibrary.Normal` (- (`self.K2_GetActorLocation`) (`local.Hit Actor Location`)))))))

(fn `OnCollision`
  (params (score :type Integer))
  (`KismetSystemLibrary.PrintString` "on collision does shit"))

(fn `Trigger Chaos Explosion`
  (params (HitDirection :type "Vector Structure"))
  (bind _exploder (`self.Exploder`))
  (bind _returnvalue (- (`SceneComponent.K2_GetComponentLocation` (`self.GeometryCollection`)) (* (`local.HitDirection`) (`KismetMathLibrary.RandomFloatInRange` 30.0 40.0))))
  (bind _returnvalue_2 (`RadialFalloff.SetRadialFalloff` (`self.RadialFalloff`) 9999999.0 0.0 1.0 0.0 (`self.Explosion Strength`) _returnvalue "Field_FallOff_None"))
  (`FieldSystemComponent.ApplyPhysicsField` _exploder true "Field_ExternalClusterStrain" null _returnvalue_2)
  (`FieldSystemComponent.ApplyPhysicsField` _exploder true "Field_LinearVelocity" null (`CullingField.SetCullingField` (`self.CullingField`) _returnvalue_2 (`RadialVector.SetRadialVector` (`self.RadialVector`) (`self.Explosion Strength`) _returnvalue) "Field_Culling_Outside")))

(fn `UserConstructionScript`
  (`parent.UserConstructionScript`))