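; BP_Obstacle is an obstacle actor that travels along a Direction vector at a random speed.
; The construction script gives it a random uniform scale between Min and Max.
; BeginPlay picks the speed and sets the ProjectileMovement velocity from it.
; Tick is empty; manual offset movement and optional random rotation logic remain as disconnected nodes.
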(event `self.ReceiveBeginPlay`
  (bind _projectilemovement (`self.ProjectileMovement`))
  (bind _projectilemovement_2 (`self.ProjectileMovement`))
  (bind _output_get (set `ProjectileMovementComponent.MaxSpeed` (`KismetMathLibrary.RandomFloatInRange` 300.0 700.0) _projectilemovement))
  (set `ProjectileMovementComponent.InitialSpeed` _output_get _projectilemovement)
  (set `MovementComponent.Velocity` (* (`ProjectileMovementComponent.InitialSpeed` _projectilemovement_2) (`self.Direction`)) _projectilemovement_2))

(event `self.ReceiveTick`
  (params (DeltaSeconds :type "Float (single-precision)")))

(fn `UserConstructionScript`
  (`self.SetActorScale3D` (`KismetMathLibrary.Conv_DoubleToVector` (`KismetMathLibrary.RandomFloatInRange` (`self.Min`) (`self.Max`)))))