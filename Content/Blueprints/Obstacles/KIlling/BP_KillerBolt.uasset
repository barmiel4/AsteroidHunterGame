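; BP_KillerBolt is an obstacle actor that destroys certain projectiles and mines that enter its Box volume.
; On the Box's begin overlap, a Sequence tries casts to BP_RifleBolt, BP_ShotgunBolt, BP_Mine and BP_UltraBolt, destroying whichever valid actor matches.
; Other overlapping actors are ignored, and BeginPlay, Tick and the construction script hold no logic.
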(event `self.Box.OnComponentBeginOverlap`
  (params (OverlappedComponent :type "PrimitiveComponent Object Reference") (OtherActor :type "Actor Object Reference") (OtherComp :type "PrimitiveComponent Object Reference") (OtherBodyIndex :type Integer) (bFromSweep :type Boolean) (SweepResult :type "HitResult Structure (by ref)"))
  (`|ExecutionSequence`
    (:`then_0`
      (bind _asbp_rifle (cast `/Game/Blueprints/Player/GUNS/BP_RifleBolt` OtherActor))
      (`/Engine/EditorBlueprintResources/StandardMacros.IsValid` _asbp_rifle
        (:`Is Valid`
          (`self.K2_DestroyActor` _asbp_rifle))))
    (:`then_1`
      (bind _asbp_shotgun (cast `/Game/Blueprints/Player/GUNS/BP_ShotgunBolt` OtherActor))
      (`/Engine/EditorBlueprintResources/StandardMacros.IsValid` _asbp_shotgun
        (:`Is Valid`
          (`self.K2_DestroyActor` _asbp_shotgun))))
    (:`then_2`
      (bind _asbp_mine (cast `/Game/Blueprints/Player/GUNS/BP_Mine` OtherActor))
      (`/Engine/EditorBlueprintResources/StandardMacros.IsValid` _asbp_mine
        (:`Is Valid`
          (`self.K2_DestroyActor` _asbp_mine))))
    (:`then_3`
      (bind _asbp_ultra_bolt (cast `/Game/Blueprints/Player/GUNS/BP_UltraBolt` OtherActor))
      (`/Engine/EditorBlueprintResources/StandardMacros.IsValid` _asbp_ultra_bolt
        (:`Is Valid`
          (`self.K2_DestroyActor` _asbp_ultra_bolt))))))

(fn `UserConstructionScript`)