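; BP_Spawner is an obstacle spawner that creates asteroids, or occasionally health pickups, at its own transform.
; On BeginPlay it starts a looping timer on Spawn, with a random interval between Min and Max rolled only once.
; Spawn creates BP_Health when a probability roll passes and health spawning is enabled, otherwise BP_Asteroid.
; The asteroid and cooler toggles appear only in unconnected showcase nodes and do not affect spawning.
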(event `self.ReceiveBeginPlay`
  (`KismetSystemLibrary.K2_SetTimer` null "Spawn" (`KismetMathLibrary.RandomFloatInRange` (`self.Min`) (`self.Max`)) true))

(fn `Spawn`
  (if (and (< (`KismetMathLibrary.RandomFloat`) (`self.HealthPickupProbablity`)) (`self.SpawnHealthPickup`))
    (`|SpawnActorFromClass` "/Game/Blueprints/Player/PICKUPS/BP_Health.BP_Health_C" (`self.GetTransform`) "Undefined" "OverrideRootScale" null null)
    (else
      (`|SpawnActorFromClass` "/Game/Blueprints/Obstacles/BP_Asteroid.BP_Asteroid_C" (`self.GetTransform`) "Undefined" "OverrideRootScale" null null))))

(fn `UserConstructionScript`)